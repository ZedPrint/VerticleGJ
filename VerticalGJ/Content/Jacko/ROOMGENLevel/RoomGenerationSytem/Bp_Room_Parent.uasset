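; Base room Blueprint for the room generation system, with side components that open up toward connected rooms.
; On BeginPlay it stores its world X and Y location as its coordinates.
; Createdpaths loops over the connected rooms, compares their coordinates to its own, and destroys the matching side component.
; A differing X selects Top or Bottom, otherwise Y selects Right or Left.
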(event `self.ReceiveBeginPlay`
  (bind (_returnvalue_x _returnvalue_y) (`KismetMathLibrary.BreakVector` (`self.K2_GetActorLocation`)))
  (set `self.Coordiantes` (`KismetMathLibrary.MakeVector2D` _returnvalue_x _returnvalue_y)))

(event `Created paths`
  (bind _coordiantes_x (`KismetMathLibrary.BreakVector2D` (`self.Coordiantes`)))
  (bind (_coordiantes_x_2 _coordiantes_y) (`KismetMathLibrary.BreakVector2D` (`self.Coordiantes`)))
  (bind _coordiantes_x_3 (`KismetMathLibrary.BreakVector2D` (`self.Coordiantes`)))
  (bind _result (`BlueprintSetLibrary.Set_ToArray` (`self.RoomConnection`)))
  (for _array_element _result
    (bind _coordiantes_x_4 (`KismetMathLibrary.BreakVector2D` (`/Game/Jacko/ROOMGENLevel/RoomGenerationSytem/Bp_Room_Parent.Coordiantes` _array_element)))
    (if (!= _coordiantes_x_4 _coordiantes_x)
      (bind _coordiantes_x_5 (`KismetMathLibrary.BreakVector2D` (`/Game/Jacko/ROOMGENLevel/RoomGenerationSytem/Bp_Room_Parent.Coordiantes` _array_element)))
      (if (> _coordiantes_x_5 _coordiantes_x_3)
        (`ActorComponent.K2_DestroyComponent` (`self.Top`))
        (else
          (`ActorComponent.K2_DestroyComponent` (`self.Bottom`))))
      (else
        (bind (_coordiantes_x_6 _coordiantes_y_2) (`KismetMathLibrary.BreakVector2D` (`/Game/Jacko/ROOMGENLevel/RoomGenerationSytem/Bp_Room_Parent.Coordiantes` _array_element)))
        (if (> _coordiantes_y_2 _coordiantes_y)
          (`ActorComponent.K2_DestroyComponent` (`self.Right`))
          (else
            (`ActorComponent.K2_DestroyComponent` (`self.Left`))))))))

(fn `UserConstructionScript`)