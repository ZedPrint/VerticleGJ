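; BP_PinHeadManager runs the PinHead section, opening the lady's dialogue and handling the end of the backrooms level.
; On BeginPlay it waits briefly, then creates and shows the WBP_PinHeadLadyTalk widget.
; The AllTextCalled event flags BackRoomsLevelCompleted on GI_PaintedGame and shows the WBP_LeaveGame widget, printing a debug message if the game instance cast fails.
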(event `self.ReceiveBeginPlay`
  (`KismetSystemLibrary.Delay` 2.0)
  (bind _returnvalue (`|CreateWidget` "/Game/Jacko/Mechanics/PinHeadSection/WBP_PinHeadLadyTalk.WBP_PinHeadLadyTalk_C"))
  (`UserWidget.AddToViewport` _returnvalue 0))

(event `AllTextCalled`
  (bind _asgi_painted_game (cast `/Game/Jacko/IMPORTANT/GI_PaintedGame` (`GameplayStatics.GetGameInstance`))
    (:`then`
      (set `/Game/Jacko/IMPORTANT/GI_PaintedGame.BackRoomsLevelCompleted` true _asgi_painted_game)
      (`KismetSystemLibrary.PrintString` "saved level ")
      (bind _returnvalue (`|CreateWidget` "/Game/Jacko/Mechanics/PinHeadSection/WBP_LeaveGame.WBP_LeaveGame_C"))
      (`UserWidget.AddToViewport` _returnvalue 0))
    (:`CastFailed`
      (`KismetSystemLibrary.PrintString` "WOMP WOMP NO SAVE"))))

(fn `UserConstructionScript`)