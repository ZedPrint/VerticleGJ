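; BP_Eyeless_Lady is an actor that can send the game to the NoEyeLady_Level map.
; On BeginPlay it runs a single sphere trace on the Visibility channel, forward from its WEIRDMAN component over TraceRange, with persistent debug drawing.
; A check for the Player tag then gates the level load.
; Tick is empty, so the trace never repeats after spawn.
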(event `self.ReceiveTick`
  (params (DeltaSeconds :type "Float (single-precision)")))

(event `self.ReceiveBeginPlay`
  (bind _weird_man (`self.WEIRD_MAN`))
  (bind _returnvalue (`SceneComponent.K2_GetComponentLocation` _weird_man))
  (`KismetSystemLibrary.SphereTraceSingle` :`Start` _returnvalue :`End` (+ _returnvalue (* (`KismetMathLibrary.GetForwardVector` (`SceneComponent.K2_GetComponentRotation` _weird_man)) (`self.TraceRange`))) :`Radius` 100.0 :`TraceChannel` "TraceTypeQuery1" :`DrawDebugType` "Persistent")
  (if (`self.ActorHasTag` "Player")
    (`GameplayStatics.OpenLevelBySoftObjectPtr` "/Game/Jamie/NoEyeLady_Level.NoEyeLady_Level")))

(fn `UserConstructionScript`)