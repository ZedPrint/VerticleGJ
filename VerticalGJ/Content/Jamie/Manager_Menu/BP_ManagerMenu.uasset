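; BP_ManagerMenu is a manager actor that decides whether to show the main menu based on level completion progress.
; On BeginPlay it reads completion flags for the Backrooms, Bathtub and Eye levels from GI_PaintedGame.
; It creates WBP_Menu and adds it to the viewport only when all three are completed, otherwise printing a debug message for the first failed check.
; An author note marks the menu branch as unfinished.
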(event `self.ReceiveBeginPlay`
  (bind _asgi_painted_game (cast `/Game/Jacko/IMPORTANT/GI_PaintedGame` (`GameplayStatics.GetGameInstance`))
    (:`then`
      (if (`/Game/Jacko/IMPORTANT/GI_PaintedGame.BackRoomsLevelCompleted` _asgi_painted_game)
        (if (`/Game/Jacko/IMPORTANT/GI_PaintedGame.BathtubLevelCompleted` _asgi_painted_game)
          (if (`/Game/Jacko/IMPORTANT/GI_PaintedGame.EyeLevelCompleted` _asgi_painted_game)
            ;[1 0 0.293] JAMIE ADD PLS (CHANGE AS WELL)
            (bind _returnvalue (`|CreateWidget` "/Game/Jamie/WBP_Menu.WBP_Menu_C"))
            (`UserWidget.AddToViewport` _returnvalue 0)
            (else
              (`KismetSystemLibrary.PrintString` "NO eye level  room  comp")))
          (else
            (`KismetSystemLibrary.PrintString` "NO Bath  room  comp")))
        (else
          (`KismetSystemLibrary.PrintString` "NO Back room  comp"))))
    (:`CastFailed`
      (`KismetSystemLibrary.PrintString` "cast failed Main menu"))))

(fn `UserConstructionScript`)